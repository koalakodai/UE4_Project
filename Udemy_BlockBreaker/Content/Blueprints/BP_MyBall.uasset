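; BP_MyBall is a ball actor that moves continuously and bounces off whatever it hits, speeding up with each hit.
; Tick moves it by Velocity times Speed and delta time, using a swept SetActorLocation.
; The Hit event mirrors Velocity across the hit normal, zeroes Y to keep the direction in the XZ plane, and raises Speed by a fixed step with no cap.
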(event `self.ReceiveHit`
  (params (MyComp :type "PrimitiveComponent Object Reference") (Other :type "Actor Object Reference") (OtherComp :type "PrimitiveComponent Object Reference") (bSelfMoved :type Boolean) (HitLocation :type "Vector Structure") (HitNormal :type "Vector Structure") (NormalImpulse :type "Vector Structure") (Hit :type "HitResult Structure (by ref)"))
  (set `self.Velocity` (`KismetMathLibrary.MakeVector` (.x (`KismetMathLibrary.MirrorVectorByNormal` (`self.Velocity`) HitNormal)) 0.0 (.z (`KismetMathLibrary.MirrorVectorByNormal` (`self.Velocity`) HitNormal))))
  (set `self.Speed` (+ (`self.Speed`) 200)))

(event `self.ReceiveTick`
  (params (DeltaSeconds :type "Float (single-precision)"))
  (`self.K2_SetActorLocation` (+ (`self.K2_GetActorLocation`) (* (* (`self.Velocity`) (`self.Speed`)) DeltaSeconds)) true))

(fn `UserConstructionScript`)