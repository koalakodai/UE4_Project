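; BP_Cube is a tutorial actor: a moving cube that damages the ball and can be blown up by key press.
; Tick nudges it along world X without sweep or delta-time scaling, and Hit calls AddDamage on any BP_Ball.
; Pressing P destroys it with a collapse sound and explosion particle.
; AddScore only increments and prints a literal zero, is not called here, and leaves the Score variable unused.
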(event `self.ReceiveHit`
  (params (MyComp :type "PrimitiveComponent Object Reference") (Other :type "Actor Object Reference") (OtherComp :type "PrimitiveComponent Object Reference") (bSelfMoved :type Boolean) (HitLocation :type "Vector Structure") (HitNormal :type "Vector Structure") (NormalImpulse :type "Vector Structure") (Hit :type "HitResult Structure (by ref)"))
  (bind _asbp_ball (cast `/Game/Tutrial/BP_Ball` Other))
  (`/Game/Tutrial/BP_Ball.AddDamage` _asbp_ball))

(event `self.ReceiveTick`
  (params (DeltaSeconds :type "Float (single-precision)"))
  (`self.K2_SetActorLocation` (+ (`self.K2_GetActorLocation`) (1.0 0.0 0.0))))

(event `Key|P`
  (params (Key :type "Key Structure"))
  (bind _returnvalue (`self.K2_GetActorLocation`))
  (:`Pressed`
    (`self.K2_DestroyActor`)
    (`GameplayStatics.PlaySoundAtLocation` "/Game/StarterContent/Audio/Collapse01.Collapse01" _returnvalue (struct) 1.0 1.0 0.0 null null null)
    (`GameplayStatics.SpawnEmitterAtLocation` "/Game/StarterContent/Particles/P_Explosion.P_Explosion" _returnvalue)))

(fn `Add Score`
  (returns (outValue :type Integer))
  (bind _result (`/Engine/EditorBlueprintResources/StandardMacros.IncrementFloat` (`KismetMathLibrary.Conv_IntToDouble` 0))
    (:`  `
      (`KismetSystemLibrary.PrintString` (`KismetStringLibrary.Conv_DoubleToString` _result))
      (return (`KismetMathLibrary.FTrunc` _result)))))

(fn `UserConstructionScript`)